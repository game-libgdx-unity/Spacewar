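; SketchCharacterBP is a character Blueprint that plays a movement sound while the forward key is held.
; BeginPlay adds an audio component at runtime, assigns it the Player_movement sound and stores it as AccelerationAudioComponent.
; Tick polls player controller 0 directly for W or Up, starting the sound if it is not already playing and stopping it when neither key is down.
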(event EventTick
  (params (DeltaSeconds :type Float%20%28single-precision%29))
  (bind _returnvalue (Game|GetPlayerController 0))
  (bind _accelerationaudiocomponent (Variables|Default|GetAccelerationAudioComponent))
  ;[1 1 1] Play acceleration sound
  (if (or (Game|Player|IsInputKeyDown _returnvalue "W") (Game|Player|IsInputKeyDown _returnvalue "Up"))
    (if (not (Audio|Components|Audio|IsPlaying (Variables|Default|GetAccelerationAudioComponent)))
      (Audio|Components|Audio|Play _accelerationaudiocomponent 0.0))
    (else
      (Audio|Components|Audio|Stop _accelerationaudiocomponent))))

(event EventBeginPlay
  ;[1 1 1] Create audio component
  (bind _returnvalue (AddComponent|AddAudioComponent false))
  (Audio|Components|Audio|SetSound _returnvalue "/Game/SoundFX/player_movement.player_movement")
  (Variables|Default|SetAccelerationAudioComponent _returnvalue))

(fn ConstructionScript)