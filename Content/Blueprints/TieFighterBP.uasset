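; TIE fighter enemy actor that handles its own entrance audio and death effect.
; On BeginPlay it adds an audio component and plays the entrance sound.
; When destroyed, it spawns an ExplosionBP at its location, slightly larger than the fighter's scale, and randomly picks one of two explosion sprites.
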(event EventBeginPlay
  ;[1 1 1] Play enemy intro music
  (bind _returnvalue (AddComponent|AddAudioComponent false))
  (Audio|Components|Audio|SetSound _returnvalue "/Game/SoundFX/tie_fighter_enterance.tie_fighter_enterance")
  (Audio|Components|Audio|Play _returnvalue 0.0))

(event EventDestroyed
  ;[1 1 1] Spawn Explosion
  (bind _returnvalue (Game|SpawnActorfromClass "/Game/Blueprints/ExplosionBP.ExplosionBP_C" (Math|Transform|MakeTransform (Transformation|GetActorLocation) "0, 0, 0" (* (Transformation|GetActorScale3D) "1.200000,1.200000,1.200000")) "AlwaysSpawn" 0 0))
  (if (Math|Random|RandomBool)
    (Rendering|Components|Sprite|SetSprite (Variables|/Game/Blueprints/ExplosionBP.ExplosionBP_C|GetSpriteComponent _returnvalue) "/Game/Sprites/Explosion1.Explosion1")
    (else
      (Rendering|Components|Sprite|SetSprite (Variables|/Game/Blueprints/ExplosionBP.ExplosionBP_C|GetSpriteComponent _returnvalue) "/Game/Sprites/Explosion2.Explosion2"))))

(fn ConstructionScript)